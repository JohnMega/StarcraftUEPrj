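; BP_OTOManager handles the end of a One-to-One (OTO) match and shows the round end screen.
; GameEndingHandleOuter has the game instance clear some widgets, pauses the game, and compares Blue and Red scores read from the WBP_OTOScore widget.
; It passes a team to OTOGameEndingHandle, which disables player 0's input and reveals WBP_OTORoundEndScreen with that team's text.
; Both widgets are found by class lookup.
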(event Custom|GameEndingHandleOuter
  (bind _foundwidgets (Widget|GetAllWidgetsOfClass "/Game/Blueprints/UI/OneToOneWidgets/Score/WBP_OTOScore.WBP_OTOScore_C" true))
  (bind _asscgame_instance (Utilities|Casting|CastToSCGameInstance (Game|GetGameInstance)))
  (Class|SCGameInstance|DeleteSomeWidgetsWhileNetworkFailure _asscgame_instance)
  (Game|SetGamePaused true)
  (if (> (Variables|/Script/StarCraft.OTOScoreWB|GetBlueTeamScore (Utilities|Array|Get(acopy) _foundwidgets)) (Variables|/Script/StarCraft.OTOScoreWB|GetRedTeamScore (Utilities|Array|Get(acopy) _foundwidgets)))
    (Class|OTOManager|OTOGameEndingHandle "BLUE_TEAM_TYPE")
    (else
      (Class|OTOManager|OTOGameEndingHandle "RED_TEAM_TYPE"))))

(event EventBeginPlay)

(event Collision|EventActorBeginOverlap
  (params (OtherActor :type Actor%20Object%20Reference)))

(event EventTick
  (params (DeltaSeconds :type Float%20%28single-precision%29)))

(event EventOTOGameEndingHandle
  (params (TeamType :type ETeamType%20Enum :default "BLUE_TEAM_TYPE"))
  (Input|DisableInput (Game|Player|GetPlayerPawn 0) (Game|GetPlayerController 0))
  (bind _foundwidgets (Widget|GetAllWidgetsOfClass "/Game/Blueprints/UI/OneToOneWidgets/RoundEndScreen/WBP_OTORoundEndScreen.WBP_OTORoundEndScreen_C" true))
  (Default|SetTeamText (Utilities|Array|Get(acopy) _foundwidgets) TeamType)
  (Widget|SetVisibility (Utilities|Array|Get(acopy) _foundwidgets) "Visible"))

(fn ConstructionScript)