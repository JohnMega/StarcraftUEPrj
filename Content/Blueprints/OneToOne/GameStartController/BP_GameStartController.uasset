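; BP_GameStartController is an actor that shows a waiting-for-players screen in a one-to-one match.
; On BeginPlay it adds WBP_OTOPlayersWait to the viewport if a game mode is valid, as on the server, and otherwise destroys itself.
; It polls the game mode's player count every Tick, then removes the widget and destroys itself when exactly two players are present.
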(event EventBeginPlay
  (Utilities|IsValid (Game|GetGameMode)
    (:Is%20Valid
      (bind _returnvalue (UserInterface|CreateWidget "/Game/Blueprints/UI/OneToOneWidgets/PlayersWait/WBP_OTOPlayersWait.WBP_OTOPlayersWait_C"))
      (Variables|Default|SetPlayerWaitWidget _returnvalue)
      (UserInterface|Viewport|AddtoViewport _returnvalue 0))
    (:Is%20Not%20Valid
      (Actor|DestroyActor))))

(event Collision|EventActorBeginOverlap
  (params (OtherActor :type Actor%20Object%20Reference)))

(event EventTick
  (params (DeltaSeconds :type Float%20%28single-precision%29))
  (Utilities|IsValid (Game|GetGameMode)
    (:Is%20Valid
      (bind _returnvalue (Class|GameModeBase|GetNumPlayers (Game|GetGameMode)))
      (if (== _returnvalue 2)
        (Widget|RemovefromParent (Variables|Default|GetPlayerWaitWidget))
        (Actor|DestroyActor)))))

(fn ConstructionScript)