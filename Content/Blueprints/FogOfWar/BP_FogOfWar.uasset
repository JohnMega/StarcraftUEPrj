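; Fog of war actor that records where units have been by painting their positions into render targets.
; BeginPlay clears the trace render target to black.
; DrawTraceonFogOfWar runs a vertical line trace through the unit's location and converts the hit into a UV with FindCollisionUV.
; That UV feeds two dynamic materials, drawn into separate trace and main-circle render targets, of which only the trace target is cleared here.
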(event EventBeginPlay
  (Rendering|ClearRenderTarget2D (Variables|Default|GetFogOfWarTraceRenderTarget)))

(event Collision|EventActorBeginOverlap
  (params (OtherActor :type Actor%20Object%20Reference)))

(event EventTick
  (params (DeltaSeconds :type Float%20%28single-precision%29)))

(event EventDrawTraceonFogOfWar
  (params (UnitLocation :type Vector%20%28by%20ref%29 :default "0, 0, 0"))
  (bind _outhit (Collision|LineTraceByChannel (+ UnitLocation "0.000000,0.000000,5000.000000") (+ UnitLocation "0.000000,0.000000,-5000.000000") "TraceTypeQuery5" true 0 "None" false))
  (Rendering|Material|SetVectorParameterValue (Variables|Default|GetFogOfWarTraceMatDynamic) (Variables|Default|GetLocationParamName) (Utilities|Struct|MakeLinearColor (.x (.UV (Class|GameplayStatics|FindCollisionUV _outhit))) (.y (.UV (Class|GameplayStatics|FindCollisionUV _outhit))) 0.0 1.0) :!class /Script/Engine.MaterialInstanceDynamic)
  (Rendering|Material|SetVectorParameterValue (Variables|Default|GetFogOfWarMainCircleMatDynamic) (Variables|Default|GetLocationParamName) (Utilities|Struct|MakeLinearColor (.x (.UV (Class|GameplayStatics|FindCollisionUV _outhit))) (.y (.UV (Class|GameplayStatics|FindCollisionUV _outhit))) 0.0 1.0) :!class /Script/Engine.MaterialInstanceDynamic)
  (Rendering|DrawMaterialtoRenderTarget (Variables|Default|GetFogOfWarTraceRenderTarget) (Variables|Default|GetFogOfWarTraceMatDynamic))
  (Rendering|DrawMaterialtoRenderTarget (Variables|Default|GetFogOfWarMainCircleRenderTarget) (Variables|Default|GetFogOfWarMainCircleMatDynamic)))

(fn ConstructionScript)