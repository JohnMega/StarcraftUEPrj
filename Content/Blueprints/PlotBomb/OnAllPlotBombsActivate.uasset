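; Level actor that starts the evacuation objective once all plot bombs are active.
; On BeginPlay it binds to the all-bombs-activated event of the BP_ActivePlotBombsNumCheck actor.
; When that fires, it destroys a barrier actor and updates each top-level task window with the evacuation order.
; Inside that same loop it adds a timer widget and a goal mask widget pointed at GoalMaskActor, once per task window found.
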(event Custom|On%20All%20Bombs%20Activate
  (Actor|DestroyActor (Variables|Default|GetBarrierActor))
  (bind _foundwidgets (Widget|GetAllWidgetsOfClass "/Game/Blueprints/UI/TaskWindow/WBP_TaskWindow.WBP_TaskWindow_C" true))
  (for _array_element _foundwidgets
    (Class|TaskWindowWB|SetTaskText _array_element "Evacuate from Mar Sara before the bombs explode")
    (bind _returnvalue (UserInterface|CreateWidget "/Game/Blueprints/UI/Timer/WBP_Timer.WBP_Timer_C"))
    (UserInterface|Viewport|AddtoViewport _returnvalue 0)
    (bind _returnvalue_2 (UserInterface|CreateWidget "/Game/Blueprints/UI/GoalMask/WBP_GoalMask.WBP_GoalMask_C"))
    (Class|GoalMaskWB|InitVars _returnvalue_2 (Utilities|Struct|MakeGoalMaskInitVars (Variables|Default|GetGoalMaskActor)))
    (UserInterface|Viewport|AddtoViewport _returnvalue_2 0)))

(event EventBeginPlay
  (bind _returnvalue (Actor|GetActorOfClass "/Game/Blueprints/PlotBomb/BP_ActivePlotBombsNumCheck.BP_ActivePlotBombsNumCheck_C"))
  (EventDispatchers|BindEventtoOnAllBombsActivate _returnvalue (delegate Custom|On%20All%20Bombs%20Activate)))

(event Collision|EventActorBeginOverlap
  (params (OtherActor :type Actor%20Object%20Reference)))

(event EventTick
  (params (DeltaSeconds :type Float%20%28single-precision%29)))

(fn ConstructionScript)