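; Level-load hook actor that kicks off the demo level's cinematic and ambient audio once loading completes.
; On BeginPlay it finds the DemoLevelScriptActor and binds to its OnLoadLevelFinish event.
; When that fires, it plays the DemoLevelSequence, then finds an AmbientSound actor by class, sets its volume multiplier to full and starts playback.
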(event Custom|On%20Demo%20Level%20Load%20Finish
  (Sequencer|Player|Play (Variables|/Script/LevelSequence.LevelSequenceActor|GetSequencePlayer (Variables|Default|GetDemoLevelSequence)) :!class /Script/MovieScene.MovieSceneSequencePlayer)
  (bind _returnvalue (Actor|GetActorOfClass "/Script/Engine.AmbientSound"))
  (Audio|Components|Audio|SetVolumeMultiplier (Variables|/Script/Engine.AmbientSound|GetAudioComponent _returnvalue) 1.0 :!class /Script/Engine.AudioComponent)
  (Audio|Components|Audio|Play (Variables|/Script/Engine.AmbientSound|GetAudioComponent _returnvalue) 0.0))

(event EventBeginPlay
  (bind _returnvalue (Actor|GetActorOfClass "/Script/StarCraft.DemoLevelScriptActor"))
  (EventDispatchers|BindEventtoOnLoadLevelFinish _returnvalue (delegate Custom|On%20Demo%20Level%20Load%20Finish)))

(event Collision|EventActorBeginOverlap
  (params (OtherActor :type Actor%20Object%20Reference)))

(event EventTick
  (params (DeltaSeconds :type Float%20%28single-precision%29)))

(fn ConstructionScript)