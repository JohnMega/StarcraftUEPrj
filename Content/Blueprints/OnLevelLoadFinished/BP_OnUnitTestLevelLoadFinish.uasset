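; Actor that sets up the UI and music for the unit test level once its loading finishes.
; On BeginPlay it finds the DemoLevelScriptActor and binds to its load-finish event.
; When that fires, it shows the level start widget, plays the level music and adds a goal mask widget initialized with the level's BP_GoalMaskActor.
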(event Custom|On%20Demo%20Level%20Load%20Finish
  (bind _returnvalue (UserInterface|CreateWidget "/Game/Blueprints/UI/WBP_UnitTestLevelStart.WBP_UnitTestLevelStart_C"))
  (UserInterface|Viewport|AddtoViewport _returnvalue 0)
  (Audio|PlaySound2D (Variables|Default|GetUnitTestLevelMusic) 1.0 1.0 0.0 0 0)
  (bind _returnvalue_2 (UserInterface|CreateWidget "/Game/Blueprints/UI/GoalMask/WBP_GoalMask.WBP_GoalMask_C"))
  (bind _returnvalue_3 (Actor|GetActorOfClass "/Game/Blueprints/UI/GoalMask/BP_GoalMaskActor.BP_GoalMaskActor_C"))
  (Class|GoalMaskWB|InitVars _returnvalue_2 (Utilities|Struct|MakeGoalMaskInitVars _returnvalue_3))
  (UserInterface|Viewport|AddtoViewport _returnvalue_2 0))

(event EventBeginPlay
  (bind _returnvalue (Actor|GetActorOfClass "/Script/StarCraft.DemoLevelScriptActor"))
  (EventDispatchers|BindEventtoOnLoadLevelFinish _returnvalue (delegate Custom|On%20Demo%20Level%20Load%20Finish)))

(event Collision|EventActorBeginOverlap
  (params (OtherActor :type Actor%20Object%20Reference)))

(event EventTick
  (params (DeltaSeconds :type Float%20%28single-precision%29)))

(fn ConstructionScript)